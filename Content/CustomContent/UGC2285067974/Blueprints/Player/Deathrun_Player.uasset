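; Per-player KJMod proxy for a Deathrun mode with Runner and Death teams, handling HUD, spawn, death and movement speed.
; The server strips weapons, gates damage by game phase and reports deaths to the gamemode proxy.
; RepNotifies and events update local HUD and round report widgets, plus each remote player's info widget.
; A throttled Tick check shows the looked-at player's info, while E triggers a server line trace for interaction.
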(event `self.Initialised`
  (bind _returnvalue (`GameplayStatics.GetPlayerController` 0))
  ;[0 1 1 0.2] On Player Initialised
  (`/Game/CustomContent/UGC2285067974/Blueprints/Deathrun_MacroLibrary.HandleClientServerLogic`
    (:`Server`
      ;;[1 1 1] Server side - Remove all tools and guns
      (`self.PrintDebugMessage` "[PlayerBP] Executed on server" (`self.WarningColor`) (/ (`self.DefaultDebugTime`) 2.0))
      (`self.SetDefaultToolAndGunSettings` (make `KJModPlayerProxyDefaultToolAndGunSetting` "NoToolsOrGuns")))
    (:`Client`
      (`self.PrintDebugMessage` "[PlayerBP] Initialising Widgets & Variables" (`self.WarningColor`) (/ (`self.DefaultDebugTime`) 2.0))
      (`|ExecutionSequence`
        (:`then_0`
          ;;[1 1 1] Local Widgets
          (`self.IsLocalOrRemote`
            (:`Local`
              (bind _returnvalue_2 (`|CreateWidget` "/Game/CustomContent/UGC2285067974/Blueprints/Interface/LocalPlayerHUD.LocalPlayerHUD_C" _returnvalue))
              (bind _output_get (set `self.LocalPlayerHUD` _returnvalue_2))
              (bind _returnvalue_3 (`|CreateWidget` "/Game/CustomContent/UGC2285067974/Blueprints/Interface/RoundReport.RoundReport_C" _returnvalue self _output_get))
              (set `self.LocalRoundReport` _returnvalue_3))))
        (:`then_1`
          ;;[1 1 1] RemoteWidgets
          (`self.IsLocalOrRemote`
            (:`Remote`
              (bind _returnvalue_4 (`|CreateWidget` "/Game/CustomContent/UGC2285067974/Blueprints/Interface/RemotePlayerInfoHUD.RemotePlayerInfoHUD_C" (`GameplayStatics.GetPlayerController` 0)))
              (set `self.RemotePlayerHUD` _returnvalue_4))))
        (:`then_2`
          ;;[1 1 1] Welcome Window & headline display (both Client & remote)
          (`self.IsLocalOrRemote`
            (:`Local`
              (bind _returnvalue_5 (`|CreateWidget` "/Game/CustomContent/UGC2285067974/Blueprints/Interface/WelcomeWindow.WelcomeWindow_C" (`GameplayStatics.GetPlayerController` 0) self (`self.LocalPlayerHUD`)))
              (bind _output_get_2 (set `self.WelcomeWindow` _returnvalue_5))
              (`UserWidget.AddToViewport` _output_get_2 0)
              (`self.SetInputMode` "UserInterfaceFocused" _output_get_2))))
        (:`then_3`
          ;;[1 1 1] Enable custom inputs
          (`self.EnableInput` (`GameplayStatics.GetPlayerController` 0)))
        (:`then_4`
          ;;[1 1 1] Register Scoreboard
          (`self.RegisterScoreboardWidget` "/Game/CustomContent/UGC2285067974/Blueprints/Interface/ScoreBoard/Scoreboard.Scoreboard_C"))
        (:`then_5`
          ;;[1 1 1] Reset Variables
          (set `self.Wins` 0)
          (set `self.Looses` 0))))))

(event `PlayerSpawnedMulticast`
  (bind _warningcolor (`self.WarningColor`))
  (bind _returnvalue (/ (`self.DefaultDebugTime`) 2.0))
  ;[1 1 1] Player Spawned Multicast
  (`self.PrintDebugMessage` "[PlayerBP] Player Spawned Multicast received" (`self.WarningColor`) (/ (`self.DefaultDebugTime`) 2.0))
  (`/Game/CustomContent/UGC2285067974/Blueprints/Deathrun_MacroLibrary.HandleClientServerLogic`
    (:`Server`
      (`self.PrintDebugMessage` "[PlayerBP] Player Spawned Multicast SERVER, ignoring" _warningcolor _returnvalue))
    (:`Client`
      (`self.PrintDebugMessage` "[PlayerBP] Player Spawned Multicast CLIENT, accepted" _warningcolor _returnvalue)
      (`self.IsLocalOrRemote`
        (:`Local`
          (`UserWidget.AddToViewport` (`self.LocalPlayerHUD`) 0)
          ;[1 1 1] Set all chats Settings
          (`self.SetChatSettings` (make `KJModPlayerProxyChatSettings` true true false 0 "" (struct :`R` 1.0 :`G` 1.0 :`B` 1.0 :`A` 1.0) (0.0 -175.0)))
          (`self.SetVoiceSettings` (make `KJModPlayerProxyVoiceSettings` true true false false)))
        (:`Remote`
          (`self.PrintDebugMessage` "[PlayerBP] Player Spawned Multicast REMOTE PLAYER" (`self.WarningColor`) (/ (`self.DefaultDebugTime`) 2.0))
          ;[1 1 1] Set Player name on remoteHUD
          (`TextBlock.SetText` (`/Game/CustomContent/UGC2285067974/Blueprints/Interface/RemotePlayerInfoHUD.PlayerNameText` (`self.RemotePlayerHUD`)) (`KismetTextLibrary.Conv_StringToText` (`self.PlayerName`))))))))

(event `self.PlayerSpawnedWithPawn`
  ;[1 0.5 0 0.2] Player spawned Pawn available, attach proxy to it and teleport Deaths to their spawn
  (`self.K2_AttachToActor` (`self.playerPawn`) "None" "SnapToTarget" "SnapToTarget" "SnapToTarget")
  (`self.K2_SetActorRelativeTransform` (`KismetMathLibrary.MakeTransform` (0.0 0.0 0.0)) false true))

(event `SetPhaseTime`
  (params (`Time in Seconds` :type Integer))
  ;[1 1 1] Set Phase Time (on LocalPlayerHUD)
  (`/Game/CustomContent/UGC2285067974/Blueprints/Deathrun_MacroLibrary.HandleClientServerLogic`
    (:`Client`
      (`/Game/CustomContent/UGC2285067974/Blueprints/Interface/LocalPlayerHUD.Set Timer Value` (`self.LocalPlayerHUD`) `Time in Seconds`))))

(event `Freze Player`
  (params (`On/Off` :type Boolean))
  ;[1 1 1] Freze player
  (`/Game/CustomContent/UGC2285067974/Blueprints/Deathrun_MacroLibrary.HandleClientServerLogic`
    (:`Client`
      (`self.SetPlayerFrozen` `On/Off`))))

(event `self.ReceiveTick`
  (params (DeltaSeconds :type "Float (single-precision)"))
  ;[1 0 1 0.2] Event tick - Chack if looking at another player, if so display info about this player
  (`/Game/CustomContent/UGC2285067974/Blueprints/Deathrun_MacroLibrary.HandleClientServerLogic`
    (:`Client`
      (`self.IsLocalOrRemote`
        (:`Local`
          (bind _output_get (set `self.TestPlayerInViewTimeout` (- (`self.TestPlayerInViewTimeout`) DeltaSeconds)))
          (if (< _output_get 0.0)
            (set `self.TestPlayerInViewTimeout` 0.2)
            (`/Engine/EditorBlueprintResources/StandardMacros.IsValid` (`self.CurrentRemotePlayerHUD`)
              (:`Is Valid`
                (`Widget.RemoveFromParent` (`self.CurrentRemotePlayerHUD`))
                (set `self.CurrentRemotePlayerHUD` null))
              (:`Is Not Valid`
                _))
            (bind _returnvalue (`self.IsPlayerLookingAtAnotherPlayer` 3000))
            (`/Engine/EditorBlueprintResources/StandardMacros.IsValid` _returnvalue
              (:`Is Valid`
                (bind _asdeathrun_player (cast `/Game/CustomContent/UGC2285067974/Blueprints/Player/Deathrun_Player` _returnvalue))
                (bind _output_get_2 (set `self.CurrentRemotePlayerHUD` (`/Game/CustomContent/UGC2285067974/Blueprints/Player/Deathrun_Player.RemotePlayerHUD` _asdeathrun_player)))
                (`UserWidget.AddToViewport` _output_get_2 0)))))))))

(event `PlayerHasDiedMulticast`
  (bind _warningcolor (`self.WarningColor`))
  (bind _returnvalue (/ (`self.DefaultDebugTime`) 2.0))
  ;[1 1 1] Player has died Multicast
  (`self.PrintDebugMessage` "[Player BP] Player has died Multicast received" (`self.WarningColor`) (/ (`self.DefaultDebugTime`) 2.0))
  (`/Game/CustomContent/UGC2285067974/Blueprints/Deathrun_MacroLibrary.HandleClientServerLogic`
    (:`Server`
      (`self.PrintDebugMessage` "[PlayerBP] Player has died Multicast SERVER, ignoring" _warningcolor _returnvalue))
    (:`Client`
      (`self.PrintDebugMessage` "[PlayerBP] Player has died Multicast CLIENT, accepted" _warningcolor _returnvalue))))

(event `ShowRoundReport`
  (params (WinnerTeam :type "/Game/CustomContent/UGC2285067974/Blueprints/Player/Deathrun_TeamsEnum Enum" :default "NewEnumerator0") (TotalPlayers :type Integer) (TotalDeaths :type Integer) (RoundTime :type Integer) (AdditionalMessage :type String))
  (bind _localplayerhud (`self.LocalPlayerHUD`))
  (bind _localroundreport (`self.LocalRoundReport`))
  (bind (_days _hours _minutes _seconds) (`KismetMathLibrary.BreakTimespan` (`KismetMathLibrary.MakeTimespan` 0 0 0 RoundTime)))
  ;[1 1 1] Round Report
  (`/Game/CustomContent/UGC2285067974/Blueprints/Deathrun_MacroLibrary.HandleClientServerLogic`
    (:`Client`
      ;;[1 1 1] Change scoreboard stats
      (if (== (`self.PlayerTeam`) WinnerTeam)
        (`/Engine/EditorBlueprintResources/StandardMacros.IncrementInt` (`self.Wins`)
          (:`  `
            _))
        (else
          (`/Engine/EditorBlueprintResources/StandardMacros.IncrementInt` (`self.Looses`)
            (:`  `
              _))))
      ;;[1 1 1] Set round report title
      (`Border.SetBrushColor` (`/Game/CustomContent/UGC2285067974/Blueprints/Interface/RoundReport.WinnerBackground` (`self.LocalRoundReport`)) (select `/Game/CustomContent/UGC2285067974/Blueprints/Player/Deathrun_TeamsEnum` WinnerTeam :`NewEnumerator0` (`self.UnknownColor`) :`NewEnumerator1` (`self.RunnerColor`) :`NewEnumerator2` (`self.DeathColor`)))
      (`TextBlock.SetText` (`/Game/CustomContent/UGC2285067974/Blueprints/Interface/RoundReport.WinnerText` (`self.LocalRoundReport`)) (select `/Game/CustomContent/UGC2285067974/Blueprints/Player/Deathrun_TeamsEnum` WinnerTeam :`NewEnumerator0` "Nobody won ?" :`NewEnumerator1` "Runners Win the Match !" :`NewEnumerator2` "Deaths Win the Match !" :!type "Text"))
      ;;[1 1 1] Set game stats
      (`TextBlock.SetText` (`/Game/CustomContent/UGC2285067974/Blueprints/Interface/RoundReport.GameStatText` (`self.LocalRoundReport`)) (`KismetTextLibrary.Conv_StringToText` (`KismetStringLibrary.Concat_StrStr` (`KismetStringLibrary.Conv_IntToString` TotalPlayers) " players took part, " (`KismetStringLibrary.Conv_IntToString` TotalDeaths) " were Deaths")))
      ;;[1 1 1] Set Round time
      (`TextBlock.SetText` (`/Game/CustomContent/UGC2285067974/Blueprints/Interface/RoundReport.RoundTimeText` (`self.LocalRoundReport`)) (`KismetTextLibrary.Conv_StringToText` (`KismetStringLibrary.Concat_StrStr` "The round latested " (`KismetStringLibrary.Right` (`KismetStringLibrary.Concat_StrStr` "0" (`KismetStringLibrary.Conv_IntToString` _minutes)) 2) ":" (`KismetStringLibrary.Right` (`KismetStringLibrary.Concat_StrStr` "0" (`KismetStringLibrary.Conv_IntToString` _seconds)) 2))))
      ;;[1 1 1] Set additional message
      (`RichTextBlock.SetText` (`/Game/CustomContent/UGC2285067974/Blueprints/Interface/RoundReport.GameRemarkText` (`self.LocalRoundReport`)) (`KismetTextLibrary.Conv_StringToText` AdditionalMessage))
      ;;[1 1 1] Show round over on player HUD
      (`|ExecutionSequence`
        (:`then_0`
          (`Border.SetBrushColor` (`/Game/CustomContent/UGC2285067974/Blueprints/Interface/LocalPlayerHUD.TeamBackground` _localplayerhud) (`self.UnknownColor`)))
        (:`then_1`
          (`TextBlock.SetText` (`/Game/CustomContent/UGC2285067974/Blueprints/Interface/LocalPlayerHUD.TeamText` _localplayerhud) "Round Over")
          (`KismetSystemLibrary.Delay` 2.0)
          ;;[1 1 1] Hide player HUD and show report
          (`Widget.RemoveFromParent` (`self.LocalPlayerHUD`))
          (`UserWidget.AddToViewport` _localroundreport 0)
          (`self.SetInputMode` "UserInterfaceFocused" _localroundreport)
          ;[1 1 1] If player never closed welcome window
          (if (`Widget.IsInViewport` (`self.WelcomeWindow`))
            (`Widget.RemoveFromParent` (`self.WelcomeWindow`))))))))

(event `HideRoundReport`
  ;[1 1 1] Round Report
  (`/Game/CustomContent/UGC2285067974/Blueprints/Deathrun_MacroLibrary.HandleClientServerLogic`
    (:`Client`
      ;;[1 1 1] Hide report and show player HUD
      (`Widget.RemoveFromParent` (`self.LocalRoundReport`))
      (`UserWidget.AddToViewport` (`self.LocalPlayerHUD`) 0)
      ;;[1 1 1] Show player game is preparing
      (`Border.SetBrushColor` (`/Game/CustomContent/UGC2285067974/Blueprints/Interface/LocalPlayerHUD.TeamBackground` (`self.LocalPlayerHUD`)) (`self.UnknownColor`))
      (`TextBlock.SetText` (`/Game/CustomContent/UGC2285067974/Blueprints/Interface/LocalPlayerHUD.TeamText` (`self.LocalPlayerHUD`)) "Preparing")
      ;;[1 1 1] Set timer to 0
      (set `/Game/CustomContent/UGC2285067974/Blueprints/Interface/LocalPlayerHUD.TimerInSeconds` 0 (`self.LocalPlayerHUD`))
      (`self.SetInputMode` "GameFocused"))))

(event `SetPlayerMovementScope`
  (params (`Player Team` :type "/Game/CustomContent/UGC2285067974/Blueprints/Player/Deathrun_TeamsEnum Enum" :default "NewEnumerator0"))
  (bind _kjmodplayerproxymovementscope (make `KJModPlayerProxyMovementScope` 800.0 500.0))
  ;[1 1 1] Change Move speed depending on your team
  (`self.SetMovementScope` (select `/Game/CustomContent/UGC2285067974/Blueprints/Player/Deathrun_TeamsEnum` `Player Team` :`NewEnumerator0` _kjmodplayerproxymovementscope :`NewEnumerator1` _kjmodplayerproxymovementscope :`NewEnumerator2` (make `KJModPlayerProxyMovementScope` 1800.0 500.0 5.6))))

(event `Key|E` :consume false
  (params (Key :type "Key Structure"))
  ;[1 1 1] Player Interact Input
  (:`Pressed`
    (if (`self.PlayerIsAlive`)
      (`self.PlayerInteractServer` (`self.playerController`) self))))

(event `PlayerInteractServer`
  (params (Controller :type "PlayerController Object Reference") (Proxy :type "/Game/CustomContent/UGC2285067974/Blueprints/Player/Deathrun_Player Object Reference"))
  (bind _returnvalue (`self.K2_GetActorLocation` (`Controller.GetViewTarget` Controller)))
  ;[1 1 1] Player Interact Server
  (bind _outhit (`KismetSystemLibrary.LineTraceSingleForObjects` :`Start` _returnvalue :`End` (+ _returnvalue (* (`KismetMathLibrary.GetForwardVector` (`Controller.GetControlRotation` Controller)) 200.0)) :`ObjectTypes` (`|MakeArray` "ObjectTypeQuery1" "ObjectTypeQuery2" :!type "EObjectTypeQuery Enum") :`DrawDebugType` "ForDuration"))
  (`self.PrintDebugMessage` (`KismetStringLibrary.Concat_StrStr` "[PlayerBP] Player interacting with" (`KismetSystemLibrary.GetDisplayName` (`.HitActor` (`GameplayStatics.BreakHitResult` _outhit)))) (`self.EntryColor`) (`self.DefaultDebugTime`))
  (message `KJModInteractableObjectInterface.PlayerInteracting` (`.HitActor` (`GameplayStatics.BreakHitResult` _outhit)) Proxy false))

(fn `OnRep_HeadlineInfo`
  (bind _headlineinfo (`self.HeadlineInfo`))
  (bind _headline (`/Game/CustomContent/UGC2285067974/Blueprints/Interface/LocalPlayerHUD.Headline` (`self.LocalPlayerHUD`)))
  (`/Game/CustomContent/UGC2285067974/Blueprints/Deathrun_MacroLibrary.HandleClientServerLogic`
    (:`Client`
      (`self.IsLocalOrRemote`
        (:`Local`
          ;[1 1 1] Update headline info on LocalPlayerHUD (if message empty hide headline)
          (`TextBlock.SetText` _headline (`KismetTextLibrary.Conv_StringToText` _headlineinfo))
          (`Widget.SetVisibility` _headline (select `bool` (`KismetStringLibrary.NotEqual_StrStr` _headlineinfo) :`false` "Collapsed" :`true` "Visible" :!type "ESlateVisibility Enum")))))))

(fn `OnRep_PlayerHealth`
  (`/Game/CustomContent/UGC2285067974/Blueprints/Deathrun_MacroLibrary.HandleClientServerLogic`
    (:`Client`
      (`self.IsLocalOrRemote`
        (:`Local`
          ;[1 1 1] Set Local HUD Healthbar
          (`ProgressBar.SetPercent` (`/Game/CustomContent/UGC2285067974/Blueprints/Interface/LocalPlayerHUD.HealthBar` (`self.LocalPlayerHUD`)) (/ (`KismetMathLibrary.Conv_IntToDouble` (`self.PlayerHealth`)) 100.0))
          (`TextBlock.SetText` (`/Game/CustomContent/UGC2285067974/Blueprints/Interface/LocalPlayerHUD.HealthText` (`self.LocalPlayerHUD`)) (`KismetTextLibrary.Conv_IntToText` (`KismetMathLibrary.Max` (`self.PlayerHealth`)))))
        (:`Remote`
          (if (<= (`self.PlayerHealth`) 0)
            ;[1 1 1] Player has died, change remote info
            (`TextBlock.SetText` (`/Game/CustomContent/UGC2285067974/Blueprints/Interface/RemotePlayerInfoHUD.PlayerTeamText` (`self.RemotePlayerHUD`)) "Dead")
            (`TextBlock.SetColorAndOpacity` (`/Game/CustomContent/UGC2285067974/Blueprints/Interface/RemotePlayerInfoHUD.PlayerTeamText` (`self.RemotePlayerHUD`)) (make `SlateColor` (`self.UnknownColor`)))))))))

(fn `OnRep_PlayerName`
  (`/Game/CustomContent/UGC2285067974/Blueprints/Deathrun_MacroLibrary.HandleClientServerLogic`
    (:`Client`
      (`self.IsLocalOrRemote`
        (:`Remote`
          (`TextBlock.SetText` (`/Game/CustomContent/UGC2285067974/Blueprints/Interface/RemotePlayerInfoHUD.PlayerNameText` (`self.RemotePlayerHUD`)) (`KismetTextLibrary.Conv_StringToText` (`self.PlayerName`))))))))

(fn `OnRep_PlayerTeam`
  (bind _playerteam (`self.PlayerTeam`))
  (bind _playerteam_2 (`self.PlayerTeam`))
  (bind _playerteamtext (`/Game/CustomContent/UGC2285067974/Blueprints/Interface/RemotePlayerInfoHUD.PlayerTeamText` (`self.RemotePlayerHUD`)))
  (`/Game/CustomContent/UGC2285067974/Blueprints/Deathrun_MacroLibrary.HandleClientServerLogic`
    (:`Client`
      (`self.IsLocalOrRemote`
        (:`Local`
          ;[1 1 1] Change Local Info
          (`Border.SetBrushColor` (`/Game/CustomContent/UGC2285067974/Blueprints/Interface/LocalPlayerHUD.TeamBackground` (`self.LocalPlayerHUD`)) (select `/Game/CustomContent/UGC2285067974/Blueprints/Player/Deathrun_TeamsEnum` _playerteam_2 :`NewEnumerator0` (`self.UnknownColor`) :`NewEnumerator1` (`self.RunnerColor`) :`NewEnumerator2` (`self.DeathColor`)))
          (`TextBlock.SetText` (`/Game/CustomContent/UGC2285067974/Blueprints/Interface/LocalPlayerHUD.TeamText` (`self.LocalPlayerHUD`)) (select `/Game/CustomContent/UGC2285067974/Blueprints/Player/Deathrun_TeamsEnum` _playerteam_2 :`NewEnumerator0` "Preparing" :`NewEnumerator1` "Runner" :`NewEnumerator2` "Death" :!type "Text")))
        (:`Remote`
          ;[1 1 1] Change Remote info
          (`TextBlock.SetText` _playerteamtext (select `/Game/CustomContent/UGC2285067974/Blueprints/Player/Deathrun_TeamsEnum` _playerteam :`NewEnumerator0` "Unknown" :`NewEnumerator1` "Runner" :`NewEnumerator2` "Death" :!type "Text"))
          (`TextBlock.SetColorAndOpacity` _playerteamtext (select `/Game/CustomContent/UGC2285067974/Blueprints/Player/Deathrun_TeamsEnum` _playerteam :`NewEnumerator0` (make `SlateColor` (`self.UnknownColor`)) :`NewEnumerator1` (make `SlateColor` (`self.RunnerColor`)) :`NewEnumerator2` (make `SlateColor` (`self.DeathColor`)))))))))

(fn `PlayerAnyDamage`
  (params (Damage :type "Float (double-precision)") (impactPoint :type "FKJModPlayerDamagePoint Enum" :default "Head") (DamageType :type "DamageType Object Reference") (InstigatedBy :type "Controller Object Reference") (DamageCauser :type "Actor Object Reference"))
  (returns (AppliedDamage :type "Float (double-precision)") (ReturnValue :type Boolean))
  (`self.PrintDebugMessage` (`KismetStringLibrary.Concat_StrStr` (`self.PlayerName`) " took damage (probably) from a trap trigered by " (`KismetSystemLibrary.GetDisplayName` InstigatedBy)) (`self.ErrorColor`) (`self.DefaultDebugTime`))
  (bind (_applieddamage _returnvalue) (`parent.PlayerAnyDamage` (select `bool` (or (`|EnumEquality` (`/Game/CustomContent/UGC2285067974/Blueprints/Gamemode/Deathrun_Gamemode.GameState` (`self.OwningGamemodeProxy`)) "NewEnumerator5") (== (`self.OwningGamemodeProxy`) DamageCauser)) :`true` Damage) impactPoint DamageType InstigatedBy DamageCauser))
  (return _applieddamage _returnvalue))

(fn `PlayerDead`
  (params (deadPawn :type "Pawn Object Reference"))
  (returns (ReturnValue :type Boolean))
  ;[1 1 1] Player died, store dead pawn and tell server that we're dead
  (set `self.DeadPawn` deadPawn)
  (`self.PrintDebugMessage` (`KismetStringLibrary.Concat_StrStr` "[Player BP] " (`self.PlayerName`) " died") (`self.WarningColor`) (/ (`self.DefaultDebugTime`) 3.0) true)
  (`/Game/CustomContent/UGC2285067974/Blueprints/Gamemode/Deathrun_Gamemode.PlayerHasDied` (`self.OwningGamemodeProxy`) self)
  (`self.PlayerHasDiedMulticast`)
  (set `self.PlayerIsAlive` false)
  (return false))

(fn `PlayerHealthArmourChange`
  (params (healthValue :type "Float (double-precision)") (armourValue :type "Float (double-precision)"))
  (returns (ReturnValue :type Boolean))
  (bind _output_get (set `self.PlayerHealth` (`KismetMathLibrary.FCeil` healthValue)))
  (`self.PrintDebugMessage` (`KismetStringLibrary.Concat_StrStr` "[PlayerBP] Health changed, value : " (`KismetStringLibrary.Conv_IntToString` _output_get)) (`self.ErrorColor`) (`self.DefaultDebugTime`))
  (return false))

(fn `PlayerSpawned`
  (returns (ReturnValue :type Boolean))
  ;[1 1 1] Player spawned, reset variables
  (`|ExecutionSequence`
    (:`then_0`
      (set `self.PlayerHealth` 100))
    (:`then_1`
      (set `self.PlayerName` (`PlayerState.GetPlayerName` (`Controller.PlayerState` (`self.playerController`))))
      (`self.PlayerSpawnedMulticast`)
      (return false))
    (:`then_2`
      (set `self.PlayerIsAlive` true))))

(fn `PrintDebugMessage`
  (params (Message :type String) (Color :type "LinearColor Structure") (Time :type "Float (double-precision)") (`Print on screen` :type Boolean))
  ;[1 1 1] Print on both UE4 & KJM screen
  (if (`self.DebugPrintOn`)
    (`KJModProxy.PrintString_KJMod` null Message `Print on screen` true Color Time)
    (`KismetSystemLibrary.PrintString` Message `Print on screen` true Color Time)))

(fn `UserConstructionScript`)