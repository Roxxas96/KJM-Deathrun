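; Deathrun gamemode for a KJMod custom mod, running rounds of Runners against randomly chosen Deaths.
; A one-second looping timer drives a state machine from waiting through pregame, team selection, countdown, main round, winner report and reset.
; Player proxies carry team and HUD info; Deaths teleport to tagged spawns, and line-traced interactions trigger tagged buttons.
; Deaths during the main phase decide the winner; a timeout leaves the default Death victory.
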(event `self.GameModeActivated`
  ;[0 1 1 0.2] Gamemode Loaded on server
  ;;[1 1 1] Join as spectator so we can manipulate spec mode
  (`self.SetJoiningPlayersParameters` (make `KJModGameModeProxyPlayerJoinParameters` true 0.0 false 5.0 0.0))
  ;;[1 1 1] Start game by reseting vars
  (`self.SwitchToNewState` "NewEnumerator7"))

(event `self.ReceiveBeginPlay`
  ;[1 0.6078 0 0.2] State Machine
  (`KismetSystemLibrary.K2_SetTimerDelegate` (delegate `StateMachine`) 1.0 true))

(event `PlayerHasDied`
  (params (DeadPlayerProxy :type "/Game/CustomContent/UGC2285067974/Blueprints/Player/Deathrun_Player Object Reference"))
  ;[1 1 1] Player Has dien (called by PlayerBP)
  (`self.HandlePlayerDeath` DeadPlayerProxy))

(event `StateMachine`
  ;[1 0.6078 0 0.2] State Machine
  (switch `/Game/CustomContent/UGC2285067974/Blueprints/Gamemode/Deathrun_GameStateEnum` (`self.GameState`)
    (:`NewEnumerator1`
      (`self.HandleWaitinOnEnoughPlayers`))
    (:`NewEnumerator2`
      (`self.HandlePregameState`)
      (`self.CheckEnoughPlayers`))
    (:`NewEnumerator3`
      (`self.HandlePregameLockOutState`)
      (`self.CheckEnoughPlayers`))
    (:`NewEnumerator4`
      (`self.HandleSelectionState`))
    (:`NewEnumerator8`
      (`self.HandleCountDownState`)
      (`self.CheckEnoughPlayers`))
    (:`NewEnumerator5`
      (`self.HandleMainPhase`)
      (`self.CheckEnoughPlayers`))
    (:`NewEnumerator6`
      (`self.HandleWinnerPhase`))
    (:`NewEnumerator7`
      (`self.HandleGameReset`))))

(event `TeleportDeathToSpawn`
  (params (`Spawn Index` :type Integer) (`Player To Teleport` :type "/Game/CustomContent/UGC2285067974/Blueprints/Player/Deathrun_Player Object Reference"))
  ;[1 1 1] Teleport Death To Spawn
  (bind _outactors (`GameplayStatics.GetAllActorsWithTag` "DeathSpawn"))
  (if (!= (`KismetArrayLibrary.Array_Length` _outactors) 0)
    (`self.K2_SetActorLocation` (`KJModPlayerProxy.playerPawn` `Player To Teleport`) (`self.K2_GetActorLocation` (`|GetArrayItem` _outactors `Spawn Index`)) false true)
    (`self.PrintDebugMessage` (`KismetStringLibrary.Concat_StrStr` "[Gamemode] " (`PlayerState.GetPlayerName` (`KJModPlayerProxy.playerState` `Player To Teleport`)) " has been teleported to a Death spawn") (`self.ValidColor`) (/ (`self.DefaultDebugTime`) 2.0))))

(event `PlayerInteract`
  (params (`Player Proxy` :type "/Game/CustomContent/UGC2285067974/Blueprints/Player/Deathrun_Player Object Reference") (`Player Controller` :type "PlayerController Object Reference"))
  ;[1 1 1] Player Interaction
  (bind (_outhit _returnvalue) (`KismetSystemLibrary.LineTraceSingleForObjects` :`ObjectTypes` (`|MakeArray` "ObjectTypeQuery1" "ObjectTypeQuery2" :!type "EObjectTypeQuery Enum") :`DrawDebugType` "ForDuration"))
  (`self.PrintDebugMessage` (`KismetStringLibrary.Concat_StrStr` "[Gamemode] Player interacting with " (`KismetSystemLibrary.GetDisplayName` (`.HitActor` (`GameplayStatics.BreakHitResult` _outhit)))) (`self.EntryColor`) (/ (`self.DefaultDebugTime`) 2.0) true)
  (if (and (`self.ActorHasTag` (`.HitActor` (`GameplayStatics.BreakHitResult` _outhit)) "Button") _returnvalue)
    (message `KJModInteractableObjectInterface.PlayerInteracting` (`.HitActor` (`GameplayStatics.BreakHitResult` _outhit)) `Player Proxy` false)))

(fn `CheckEnoughPlayers`
  (if (< (`self.CurrentPlayerCount`) (`self.MinPlayers`))
    (bind _returnvalue (`self.GetPlayerProxies`))
    (for _array_element _returnvalue
      (bind _playerpawn (`KJModPlayerProxy.playerPawn` _array_element))
      (`/Engine/EditorBlueprintResources/StandardMacros.IsValid` _playerpawn
        (:`Is Valid`
          (`GameplayStatics.ApplyDamage` _playerpawn 100000000.0 null self))
        (:`Is Not Valid`
          _))
      (`self.SwitchToNewState` "NewEnumerator7"))))

(fn `GenerateRoundReport`
  (params (`Player Proxy` :type "/Game/CustomContent/UGC2285067974/Blueprints/Player/Deathrun_Player Object Reference"))
  (`/Game/CustomContent/UGC2285067974/Blueprints/Player/Deathrun_Player.ShowRoundReport` `Player Proxy` (`self.WinnerTeam`) (`self.TotalPlayersInRound`) (`self.TotalDeathsInRound`) (- (`self.MainRoundTime`) (`self.MainRoundTimeout`)) "Thank you for playing Deathrun ! \n \nThe round has ended"))

(fn `HandleCountDownState`
  (bind _countdowntimeout (`self.CountDownTimeout`))
  (if (== (`self.CountDownTimeout`) 0)
    ;[1 1 1] Clear headline and switch to new state
    (`self.ShowInformationtoAllPlayers` "")
    (`self.SwitchToNewState` "NewEnumerator5")
    (else
      ;[1 1 1] Handle CountDown
      (`self.ShowInformationtoAllPlayers` (`KismetStringLibrary.Concat_StrStr` "Games Starts in " (`KismetStringLibrary.Conv_IntToString` _countdowntimeout)) true)
      (`/Engine/EditorBlueprintResources/StandardMacros.DecrementInt` _countdowntimeout))))

(fn `HandleGameReset`
  (`self.PrintDebugMessage` "[Gamemode State] Game Reset Called" (`self.EntryColor`) (/ (`self.DefaultDebugTime`) 2.0))
  (`|ExecutionSequence`
    (:`then_0`
      (set `self.PregameTimeout` (`self.PreroundTime`))
      (set `self.PregameLockOutTimeout` 5) ; Do not touch
    )
    (:`then_1`
      (set `self.MainRoundTimeout` (`self.MainRoundTime`)))
    (:`then_2`
      (set `self.WinnerPhaseTimeout` (`self.WinnerPhaseTime`)))
    (:`then_3`
      (set `self.WinnerTeam` "NewEnumerator2"))
    (:`then_4`
      (`self.RoundEnd`))
    (:`then_5`
      (`self.SwitchToNewState` "NewEnumerator1"))
    (:`then_6`
      (set `self.CountDownTimeout` (`self.CountDownTime`)))))

(fn `HandleMainPhase`
  (`self.PrintDebugMessage` (`KismetStringLibrary.Concat_StrStr` "[Gamemode State] Main State, timeout : " (`KismetStringLibrary.Conv_IntToString` (`self.MainRoundTimeout`))) (`self.EntryColor`) (`self.DefaultDebugTime`))
  (bind _result (`/Engine/EditorBlueprintResources/StandardMacros.DecrementInt` (`self.MainRoundTimeout`))
    (:`  `
      (if (== _result 0)
        (`self.SwitchToNewState` "NewEnumerator6")))))

(fn `HandlePlayerDeath`
  (params (`Dead Player` :type "/Game/CustomContent/UGC2285067974/Blueprints/Player/Deathrun_Player Object Reference"))
  (locals (AnyRunnersAlive :type Boolean) (AnyDeathsAlive :type Boolean))
  ;[1 1 1] Deaths should be always on main phase
  (if (`|EnumEquality` (`self.GameState`) "NewEnumerator5")
    (`self.PrintDebugMessage` (`KismetStringLibrary.Concat_StrStr` "[Gamemode] HandlePlayerDeath, players : " (`KismetStringLibrary.Conv_IntToString` (`KismetArrayLibrary.Array_Length` (`self.PlayerInfo`)))) (`self.ValidColor`) (* (`self.DefaultDebugTime`) 1.5))
    ;[1 1 1] Get player info and tick player as dead (match his proxy in the player info table)
    (for (_array_element _array_index) (`self.PlayerInfo`)
      (if (== (`.Proxy_2_26742E674AFF48DAC01DD281DB62DC19` (break `/Game/CustomContent/UGC2285067974/Blueprints/Gamemode/Deathrun_PlayerInfo` _array_element)) `Dead Player`)
        (bind _structout (setmembers `/Game/CustomContent/UGC2285067974/Blueprints/Gamemode/Deathrun_PlayerInfo` :`StructRef` _array_element :`Alive` false))
        (`KismetArrayLibrary.Array_Set` (`self.PlayerInfo`) _array_index _structout)
        (break)))
    ;[0 0.9169 1 0.2] Detect if any Runner is alive
    (set `local.AnyRunnersAlive` false)
    (for _array_element_2 (`self.PlayerInfo`)
      (bind ((`Team_5_26FA26434F6360DAC1C5ABB554531FBE` _team) (`Alive_12_D085A29547DFD4147C97A8A8D17C9E2C` _alive)) (break `/Game/CustomContent/UGC2285067974/Blueprints/Gamemode/Deathrun_PlayerInfo` _array_element_2))
      (if (and (`|EnumEquality` _team "NewEnumerator1") _alive)
        (set `local.AnyRunnersAlive` true)
        (break)))
    ;[1 0 0 0.2] Detect if any Death is alive
    (set `local.AnyDeathsAlive` false)
    (for _array_element_3 (`self.PlayerInfo`)
      (bind ((`Team_5_26FA26434F6360DAC1C5ABB554531FBE` _team_2) (`Alive_12_D085A29547DFD4147C97A8A8D17C9E2C` _alive_2)) (break `/Game/CustomContent/UGC2285067974/Blueprints/Gamemode/Deathrun_PlayerInfo` _array_element_3))
      (if (and (`|EnumEquality` _team_2 "NewEnumerator2") _alive_2)
        (set `local.AnyDeathsAlive` true)
        (break)))
    ;[1 1 1] Runners win ?
    (if (and (`local.AnyRunnersAlive`) (not (`local.AnyDeathsAlive`)))
      (set `self.WinnerTeam` "NewEnumerator1")
      (`self.SwitchToNewState` "NewEnumerator6")
      (else
        ;[1 1 1] Deaths win ?
        (if (and (`local.AnyDeathsAlive`) (not (`local.AnyRunnersAlive`)))
          (set `self.WinnerTeam` "NewEnumerator2")
          (`self.SwitchToNewState` "NewEnumerator6")
          (else
            (`self.PrintDebugMessage` "[Gamemode] HandlePlayerDeath - no winner, game still running" (`self.ValidColor`) (/ (`self.DefaultDebugTime`) 2.0))
            (for (_array_element_4 _array_index_2) (`self.PlayerInfo`)
              (bind (_proxy _controller _team_3 _alive_3) (break `/Game/CustomContent/UGC2285067974/Blueprints/Gamemode/Deathrun_PlayerInfo` _array_element_4))
              (`self.PrintDebugMessage` (`KismetStringLibrary.Concat_StrStr` "Player ID : " (`KismetStringLibrary.Conv_IntToString` _array_index_2) " , Settings : " (`KismetStringLibrary.Concat_StrStr` (`KismetSystemLibrary.GetDisplayName` _proxy) " - " (`KismetSystemLibrary.GetDisplayName` _controller) " = " (`|GetEnumeratorNameAsString` _team_3) " / " (`KismetStringLibrary.Conv_BoolToString` _alive_3) " ...")) (`self.ValidColor`) (`self.DefaultDebugTime`)))))))))

(fn `HandlePregameLockOutState`
  (`self.PrintDebugMessage` (`KismetStringLibrary.Concat_StrStr` "[Gamemode] Pregame LockOut state, timeout : " (`KismetStringLibrary.Conv_IntToString` (`self.PregameLockOutTimeout`))) (`self.EntryColor`) (/ (`self.DefaultDebugTime`) 3.0))
  (bind _result (`/Engine/EditorBlueprintResources/StandardMacros.DecrementInt` (`self.PregameLockOutTimeout`))
    (:`  `
      (if (== _result 0)
        (`self.SwitchToNewState` "NewEnumerator4")))))

(fn `HandlePregameState`
  (`self.PrintDebugMessage` (`KismetStringLibrary.Concat_StrStr` "[Gamemode] Pregame state, timeout : " (`KismetStringLibrary.Conv_IntToString` (`self.PregameTimeout`))) (`self.EntryColor`) (/ (`self.DefaultDebugTime`) 3.0))
  (bind _result (`/Engine/EditorBlueprintResources/StandardMacros.DecrementInt` (`self.PregameTimeout`))
    (:`  `
      (if (== _result 0)
        (`self.SwitchToNewState` "NewEnumerator3")))))

(fn `HandleSelectionState`
  (`self.PrintDebugMessage` "[Gamemode State] Selection state, selecting player teams" (`self.EntryColor`) (/ (`self.DefaultDebugTime`) 3.0))
  (`self.SwitchToNewState` "NewEnumerator8"))

(fn `HandleWaitinOnEnoughPlayers`
  (if (>= (`self.CurrentPlayerCount`) (`self.MinPlayers`))
    ;[1 1 1] Enough players, hide headline info and proceede
    (`self.ShowInformationtoAllPlayers` "")
    (`self.SwitchToNewState` "NewEnumerator2")
    (set `self.WaitingOnEnoughPlayersTime` 0)
    (else
      ;[1 1 1] Show waiting info to players
      (bind _result (`/Engine/EditorBlueprintResources/StandardMacros.IncrementInt` (`self.WaitingOnEnoughPlayersTime`))
        (:`  `
          (bind (_days _hours _minutes _seconds) (`KismetMathLibrary.BreakTimespan` (`KismetMathLibrary.MakeTimespan` 0 0 0 _result)))
          (`self.ShowInformationtoAllPlayers` (`KismetStringLibrary.Concat_StrStr` "Waiting on more players (require " (`KismetStringLibrary.Conv_IntToString` (`self.MinPlayers`)) " players to start) - " (`KismetStringLibrary.Right` (`KismetStringLibrary.Concat_StrStr` "0" (`KismetStringLibrary.Conv_IntToString` _minutes)) 2) ":" (`KismetStringLibrary.Right` (`KismetStringLibrary.Concat_StrStr` "0" (`KismetStringLibrary.Conv_IntToString` _seconds)) 2)) true))))))

(fn `HandleWinnerPhase`
  (`self.PrintDebugMessage` (`KismetStringLibrary.Concat_StrStr` "[Gamemode State] Winner phase, timeout : " (`KismetStringLibrary.Conv_IntToString` (`self.WinnerPhaseTimeout`))) (`self.EntryColor`) (/ (`self.DefaultDebugTime`) 2.0))
  (bind _result (`/Engine/EditorBlueprintResources/StandardMacros.DecrementInt` (`self.WinnerPhaseTimeout`))
    (:`  `
      (if (== _result 0)
        (`self.SwitchToNewState` "NewEnumerator7")))))

(fn `PlayerHasJoined`
  (params (joiningPlayerController :type "PlayerController Object Reference"))
  (returns (ReturnValue :type "KJModPlayerProxy Object Reference"))
  ;[1 1 1] Player has joined, increment player count
  (`/Engine/EditorBlueprintResources/StandardMacros.IncrementInt` (`self.CurrentPlayerCount`)
    (:`  `
      (`self.PrintDebugMessage` (`KismetStringLibrary.Concat_StrStr` "[Gamemode] " (`AdvancedSessionsLibrary.GetPlayerName` joiningPlayerController) " has joined the game") (`self.EntryColor`) (/ (`self.DefaultDebugTime`) 2.0) true)
      ;[1 1 1] Spawn player proxy, initialise it and add it to the representation
      (bind _returnvalue (`|SpawnActorFromClass` "/Game/CustomContent/UGC2285067974/Blueprints/Player/Deathrun_Player.Deathrun_Player_C" (`KismetMathLibrary.MakeTransform` (0.0 0.0 0.0)) "Undefined" "OverrideRootScale" joiningPlayerController self null))
      (`KismetArrayLibrary.Array_Add` (`self.PlayerRepresentation`) _returnvalue))))

(fn `PlayerHasLeft`
  (params (leavingPlayerController :type "PlayerController Object Reference"))
  (returns (ReturnValue :type Boolean))
  ;[1 1 1] Decrease player count
  (`/Engine/EditorBlueprintResources/StandardMacros.DecrementInt` (`self.CurrentPlayerCount`)
    (:`  `
      (`self.PrintDebugMessage` (`KismetStringLibrary.Concat_StrStr` "[Gamemode] " (`PlayerState.GetPlayerName` (`Controller.PlayerState` leavingPlayerController)) " has left the game") (`self.EntryColor`) (/ (`self.DefaultDebugTime`) 2.0) true)
      ;[1 1 1] Match representation with leaving player
      (for _array_element (`self.PlayerRepresentation`)
        (if (== leavingPlayerController (`KJModPlayerProxy.playerController` _array_element))
          (bind _deadpawn (`/Game/CustomContent/UGC2285067974/Blueprints/Player/Deathrun_Player.DeadPawn` _array_element))
          ;[1 1 1] Remove dead pawn
          (`/Engine/EditorBlueprintResources/StandardMacros.IsValid` _deadpawn
            (:`Is Valid`
              (`KJModPlayerProxy.RemoveDeadPawn` _array_element _deadpawn)
              (`self.HandlePlayerDeath` _array_element)
              ;[1 1 1] Remove player proxy and its representation
              (`self.K2_DestroyActor` _array_element)
              (`KismetArrayLibrary.Array_RemoveItem` (`self.PlayerRepresentation`) _array_element)
              (return false))))))))

(fn `PrintDebugMessage`
  (params (Message :type String) (Color :type "LinearColor Structure") (Time :type "Float (double-precision)") (`Print on Screen` :type Boolean))
  ;[1 1 1] Print on both UE4 & KJM screen
  (if (`self.DebugPrintOn`)
    (`KJModProxy.PrintString_KJMod` null Message `Print on Screen` true Color Time)
    (`KismetSystemLibrary.PrintString` Message `Print on Screen` true Color Time)))

(fn `SelectPlayerTeamAndTeleportDeaths`
  (locals (PlayerProxies :type "Array of KJModPlayerProxy Object Reference") (TotalPlayers :type Integer) (PlayerTeams :type "Array of /Game/CustomContent/UGC2285067974/Blueprints/Player/Deathrun_TeamsEnum Enum") (TotalDeaths :type Integer) (PreviouslySelectedIndex :type "Array of Integer"))
  (bind _returnvalue (`self.GetPlayerProxies`))
  (`self.PrintDebugMessage` (`KismetStringLibrary.Concat_StrStr` "[Gamemode] SelectPlayerTeam called, count : " (`KismetStringLibrary.Conv_IntToString` (`KismetArrayLibrary.Array_Length` (`self.PlayerInfo`))) " and " (`KismetStringLibrary.Conv_IntToString` (`KismetArrayLibrary.Array_Length` _returnvalue))) (`self.ValidColor`) (* (`self.DefaultDebugTime`) 1.5))
  ;[1 1 1] Reset Variables
  (bind _returnvalue_2 (`self.GetPlayerProxies`))
  (bind _output_get (set `local.PlayerProxies` _returnvalue_2))
  (set `local.TotalPlayers` (`KismetArrayLibrary.Array_Length` _output_get))
  (`KismetArrayLibrary.Array_Clear` (`self.PlayerInfo`))
  (`KismetArrayLibrary.Array_Clear` (`local.PlayerTeams`))
  ;[1 1 1] Fill array with innocents
  (for _ (`local.PlayerProxies`)
    (`KismetArrayLibrary.Array_Add` (`local.PlayerTeams`) "NewEnumerator1"))
  ;[1 1 1] Set number of Deaths in game
  (set `local.TotalDeaths` (`KismetMathLibrary.FFloor` (`KismetMathLibrary.FMax` (* (`local.TotalPlayers`) (`self.DeathsRatio`)) 1.0)))
  ;[1 1 1] Select a random Death
  (`KismetArrayLibrary.Array_Clear` (`local.PreviouslySelectedIndex`))
  (for _ (range (`local.TotalDeaths`))
    (bind _unique_value (`self.SelectUniqueRandomValue` (`local.PreviouslySelectedIndex`) (- (`local.TotalPlayers`) 1)))
    (`KismetArrayLibrary.Array_Add` (`local.PreviouslySelectedIndex`) _unique_value)
    (`KismetArrayLibrary.Array_Set` (`local.PlayerTeams`) _unique_value "NewEnumerator2"))
  ;[1 1 1] Clear variables of old round
  (set `self.TotalPlayersInRound` 0)
  (set `self.TotalDeathsInRound` 0)
  ;[1 1 1] Send to player his team
  (`KismetArrayLibrary.Array_Clear` (`local.PreviouslySelectedIndex`))
  (for (_array_element _array_index) (`local.PlayerProxies`)
    (bind _asdeathrun_player (cast `/Game/CustomContent/UGC2285067974/Blueprints/Player/Deathrun_Player` _array_element))
    (bind _output (`|GetArrayItem` (`local.PlayerTeams`) _array_index))
    (set `/Game/CustomContent/UGC2285067974/Blueprints/Player/Deathrun_Player.PlayerTeam` _output _asdeathrun_player)
    ;[1 1 1] Adding the player to PlayerInfo struct so we can track player state for Winner phase
    (`KismetArrayLibrary.Array_Add` (`self.PlayerInfo`) (make `/Game/CustomContent/UGC2285067974/Blueprints/Gamemode/Deathrun_PlayerInfo` _asdeathrun_player (`KJModPlayerProxy.playerController` _asdeathrun_player) _output true))
    (`self.PrintDebugMessage` "[Gamemode] Added user to PlayerInfo struct" (`self.ValidColor`) (* (`self.DefaultDebugTime`) 1.5))
    ;[1 1 1] These variables are used in end of round report
    (switch `/Game/CustomContent/UGC2285067974/Blueprints/Player/Deathrun_TeamsEnum` _output
      (:`NewEnumerator1`
        (`/Engine/EditorBlueprintResources/StandardMacros.IncrementInt` (`self.TotalPlayersInRound`) :!label _label))
      (:`NewEnumerator2`
        (`|ExecutionSequence`
          (:`then_0`
            (`/Engine/EditorBlueprintResources/StandardMacros.IncrementInt` (`self.TotalDeathsInRound`)
              (:`  `
                (goto _label))))
          (:`then_1`
            ;[1 1 1] Teleport Deaths to their Spawns
            (bind _unique_value_2 (`self.SelectUniqueRandomValue` (`local.PreviouslySelectedIndex`) (`local.TotalDeaths`)))
            (`self.TeleportDeathToSpawn` _unique_value_2 _asdeathrun_player)
            (`KismetArrayLibrary.Array_Add` (`local.PreviouslySelectedIndex`) _unique_value_2)))))))

(fn `SelectUniqueRandomValue`
  (params (`Previous Values` :type "Array of Integer") (`Max Value` :type Integer))
  (returns (`Unique Value` :type Integer))
  (locals (MaxIterations :type Integer) (UniqueNumber :type Integer) (UniqueValueFound :type Boolean))
  (set `local.MaxIterations` 32)
  (set `local.UniqueValueFound` false)
  (while (and (not (`local.UniqueValueFound`)) (> (`local.MaxIterations`) 0))
    (bind _output_get (set `local.UniqueNumber` (`KismetMathLibrary.RandomIntegerInRange` 0 `Max Value`)))
    (if (== (`KismetArrayLibrary.Array_Find` `Previous Values` _output_get) -1)
      (set `local.UniqueValueFound` true)
      (else
        (`/Engine/EditorBlueprintResources/StandardMacros.DecrementInt` (`local.MaxIterations`)))))
  (return (`local.UniqueNumber`)))

(fn `ShowInformationtoAllPlayers`
  (params (Message :type String) (Value :type Boolean))
  ;[1 1 1] Show info on player headline, visible = false or empty message will hide headline
  (bind _returnvalue (`self.GetPlayerProxies`))
  (for _array_element _returnvalue
    (bind _asdeathrun_player (cast `/Game/CustomContent/UGC2285067974/Blueprints/Player/Deathrun_Player` _array_element))
    (set `/Game/CustomContent/UGC2285067974/Blueprints/Player/Deathrun_Player.HeadlineInfo` (select `bool` Value :`true` Message) _asdeathrun_player)))

(fn `SwitchToNewState`
  (params (State :type "/Game/CustomContent/UGC2285067974/Blueprints/Gamemode/Deathrun_GameStateEnum Enum" :default "NewEnumerator0"))
  ;[1 1 1] Set new state and execute actions depending on the state
  (bind _output_get (set `self.GameState` State))
  (`self.PrintDebugMessage` (`KismetStringLibrary.Concat_StrStr` "[Gamemode] Switching to new state : " (`|GetEnumeratorNameAsString` _output_get)) (`self.EntryColor`) (/ (`self.DefaultDebugTime`) 1.5))
  (switch `/Game/CustomContent/UGC2285067974/Blueprints/Gamemode/Deathrun_GameStateEnum` (`self.GameState`)
    (:`NewEnumerator2`
      ;[1 1 1] Pregame - Spawn all players, reset their teams and set the phase timer on their localPlayerHUD
      (for _array_element (`self.PlayerRepresentation`)
        (`self.SpawnPlayer` _array_element)
        (`/Game/CustomContent/UGC2285067974/Blueprints/Player/Deathrun_Player.Freze Player` _array_element true)
        (set `/Game/CustomContent/UGC2285067974/Blueprints/Player/Deathrun_Player.PlayerTeam` "NewEnumerator0" _array_element)
        (`/Game/CustomContent/UGC2285067974/Blueprints/Player/Deathrun_Player.SetPhaseTime` _array_element (+ (`self.PreroundTime`) (`self.PregameLockOutTimeout`)))))
    (:`NewEnumerator4`
      ;[1 1 1] Selection phase
      (`self.SelectPlayerTeamAndTeleportDeaths`))
    (:`NewEnumerator5`
      ;[1 1 1] Main Phase
      (for _array_element_2 (`self.PlayerRepresentation`)
        (`/Game/CustomContent/UGC2285067974/Blueprints/Player/Deathrun_Player.SetPhaseTime` _array_element_2 (`self.MainRoundTime`))
        (`/Game/CustomContent/UGC2285067974/Blueprints/Player/Deathrun_Player.Freze Player` _array_element_2 false))
      (`self.RoundReset`))
    (:`NewEnumerator6`
      ;[1 1 1] Winner Phase - Generate round report and show it
      (for _array_element_3 (`self.PlayerRepresentation`)
        (`/Game/CustomContent/UGC2285067974/Blueprints/Player/Deathrun_Player.SetPhaseTime` _array_element_3 (`self.WinnerPhaseTime`))
        (`self.GenerateRoundReport` _array_element_3)))
    (:`NewEnumerator7`
      ;[1 1 1] Game Reset - Remove all Deat pawn, Hide Round report and End Round
      (for _array_element_4 (`self.PlayerRepresentation`)
        (`/Game/CustomContent/UGC2285067974/Blueprints/Player/Deathrun_Player.HideRoundReport` _array_element_4)
        (bind _deadpawn (`/Game/CustomContent/UGC2285067974/Blueprints/Player/Deathrun_Player.DeadPawn` _array_element_4))
        (`/Engine/EditorBlueprintResources/StandardMacros.IsValid` _deadpawn
          (:`Is Valid`
            (`KJModPlayerProxy.RemoveDeadPawn` _array_element_4 _deadpawn))))
      (`self.RoundEnd`))))

(fn `UserConstructionScript`)