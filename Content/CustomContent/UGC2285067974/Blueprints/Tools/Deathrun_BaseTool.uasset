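; Base tool for the Deathrun game mode, handling limited uses that recharge on a cooldown.
; UseTool spends a use only in one specific game state, checked through the Deathrun_Player proxy attached to the owner, and starts the cooldown timer.
; Tick restores spent uses one at a time, only while the tool is activated.
; OnRep handlers for use count and cooldown call empty, apparently overridable, Rep functions.
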(event `KJModToolProxyInterface.ToolProxy_Activated`
  ;[1 1 1] Tool activated
  (set `self.ToolActivated` true))

(event `KJModToolProxyInterface.ToolProxy_Deactivated`
  ;[1 1 1] Tool deactivated
  (set `self.ToolActivated` false))

(event `self.ReceiveTick`
  (params (DeltaSeconds :type "Float (single-precision)"))
  ;[1 1 1] Cooldown system
  (if (`self.ToolActivated`)
    (if (and (>= (`self.Cooldown`) 0.0) (> (`self.UseCount`) 0))
      (if (<= (`self.CooldownTimeout`) 0.0)
        (bind _output_get (set `self.UseCount` (- (`self.UseCount`) 1)))
        (if (> _output_get 0)
          (set `self.CooldownTimeout` (`self.Cooldown`)))
        (else
          (set `self.CooldownTimeout` (- (`self.CooldownTimeout`) DeltaSeconds)))))))

(fn `GetOwnerProxy`
  (returns (PlayerProxy :type "/Game/CustomContent/UGC2285067974/Blueprints/Player/Deathrun_Player Object Reference"))
  (for _array_element (`self.GetAttachedActors` (`self.GetOwner`) true)
    (if (== (`GameplayStatics.GetObjectClass` _array_element) "/Game/CustomContent/UGC2285067974/Blueprints/Player/Deathrun_Player.Deathrun_Player_C")
      (bind _asdeathrun_player (cast `/Game/CustomContent/UGC2285067974/Blueprints/Player/Deathrun_Player` _array_element))
      (return _asdeathrun_player))))

(fn `IsLocallyControlled`
  (returns (LocallyControlled :type Boolean))
  (bind _ascharacter (cast `Character` (`self.GetOwner`)))
  (return (`Pawn.IsLocallyControlled` _ascharacter)))

(fn `OnRep_CooldownTimeout`
  (`self.Rep_CooldownTimeout`))

(fn `OnRep_UseCount`
  (`self.Rep_UseCount`))

(fn `Rep_CooldownTimeout`)

(fn `Rep_UseCount`)

(fn `UserConstructionScript`)

(fn `UseTool`
  (returns (`Tool used` :type Boolean))
  (if (< (`self.UseCount`) (`self.MaxUses`))
    (bind _playerproxy (`self.GetOwnerProxy`))
    (if (`|EnumEquality` (`/Game/CustomContent/UGC2285067974/Blueprints/Gamemode/Deathrun_Gamemode.GameState` (`/Game/CustomContent/UGC2285067974/Blueprints/Player/Deathrun_Player.OwningGamemodeProxy` _playerproxy)) "NewEnumerator5")
      (set `self.UseCount` (+ (`self.UseCount`) 1))
      (if (<= (`self.CooldownTimeout`) 0.0)
        (set `self.CooldownTimeout` (`KismetMathLibrary.FMax` (`self.Cooldown`))))
      (return true)
      (else
        (return false)))
    (else
      (return false))))