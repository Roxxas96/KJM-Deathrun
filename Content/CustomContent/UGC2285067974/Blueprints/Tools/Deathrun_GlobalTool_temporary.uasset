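; Deathrun global player tool that grants a Shift dash and an F-key bait spawn, both gated on game state.
; Each ability tracks use count and cooldown, with Tick restoring charges over time.
; Dash moves the owner by timeline-driven SetActorLocation on server and client rather than an impulse, while bait spawns server-side at the character.
; RepNotify functions update the HUD bars, tints, dash count and the dash ribbon effect.
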(event `KJModToolProxyInterface.ToolProxy_Deactivated`
  ;[1 1 1] Reset HUD Variables when Tool Removed
  (set `self.ToolActivated` false)
  (bind _ownerplayerproxy (`self.GetOwnerPlayerProxy`)
    (:`Output`
      (`|ExecutionSequence`
        (:`then_0`
          (bind _localplayerhud (`/Game/CustomContent/UGC2285067974/Blueprints/Player/Deathrun_Player.LocalPlayerHUD` _ownerplayerproxy))
          (`Image.SetBrushTintColor` (`/Game/CustomContent/UGC2285067974/Blueprints/Interface/LocalPlayerHUD.BaitBackground` _localplayerhud) (make `SlateColor` (struct :`R` 0.1 :`G` 0.1 :`B` 0.1 :`A` 1.0))))
        (:`then_1`
          (`ProgressBar.SetPercent` (`/Game/CustomContent/UGC2285067974/Blueprints/Interface/LocalPlayerHUD.BaitBar` _localplayerhud) 0.0))
        (:`then_2`
          (`ProgressBar.SetPercent` (`/Game/CustomContent/UGC2285067974/Blueprints/Interface/LocalPlayerHUD.DashBar` _localplayerhud) 0.0))
        (:`then_3`
          (`Image.SetBrushTintColor` (`/Game/CustomContent/UGC2285067974/Blueprints/Interface/LocalPlayerHUD.DashBackground` _localplayerhud) (make `SlateColor` (struct :`R` 0.1 :`G` 0.1 :`B` 0.1 :`A` 1.0))))
        (:`then_4`
          (`Widget.SetVisibility` (`/Game/CustomContent/UGC2285067974/Blueprints/Interface/LocalPlayerHUD.DashCount` _localplayerhud) "Collapsed"))))))

(event `KJModToolProxyInterface.ToolProxy_Activated`
  ;[1 1 1] Reset vars to update HUD
  (set `self.ToolActivated` true)
  (set `self.CooldownTimeOutDash` 0.0)
  (set `self.CooldownTimeOutBait` 0.0)
  (set `self.UseCountBait` 1)
  (set `self.UseCountDash` 3))

(event `self.ReceiveBeginPlay`
  ;[1 1 1] Register
  (`/Game/CustomContent/UGC2285067974/Blueprints/Deathrun_MacroLibrary.HandleClientServerLogic`
    (:`Client`
      (`self.IsLocallyControlled`
        (:`Local`
          (`self.RegisterToolLocally`)
          (`self.ShowMessage` "Press SHIFT to dash and F to spawn the bait" 10.0 true "/Game/CustomContent/UGC2285067974/Textures/deathrun_logo512_bmp.deathrun_logo512_bmp")
          (`self.SetCustomAction` "F" "" "" 1))))))

(event `self.ReceiveTick`
  (params (DeltaSeconds :type "Float (single-precision)"))
  ;[1 1 1] CD Timeout update
  (if (`self.ToolActivated`)
    (`|ExecutionSequence`
      (:`then_0`
        ;;[1 1 1] Dash CD
        (if (and (>= (`self.CooldownDash`) 0.0) (> (`self.UseCountDash`) 0))
          (if (<= (`self.CooldownTimeOutDash`) 0.0)
            (bind _output_get (set `self.UseCountDash` (- (`self.UseCountDash`) 1)))
            (if (> _output_get 0)
              (set `self.CooldownTimeOutDash` (`self.CooldownDash`)))
            (else
              (set `self.CooldownTimeOutDash` (- (`self.CooldownTimeOutDash`) DeltaSeconds))))))
      (:`then_1`
        ;;[1 1 1] Bait CD
        (if (and (>= (`self.CooldownBait`) 0.0) (> (`self.UseCountBait`) 0))
          (if (<= (`self.CooldownTimeOutBait`) 0.0)
            (bind _output_get_2 (set `self.UseCountBait` (- (`self.UseCountBait`) 1)))
            (if (> _output_get_2 0)
              (set `self.CooldownTimeOutBait` (`self.CooldownBait`)))
            (else
              (set `self.CooldownTimeOutBait` (- (`self.CooldownTimeOutBait`) DeltaSeconds)))))))))

(event `DashServer`
  (params (LastInput :type "Vector Structure") (Owner :type "Actor Object Reference") (ToolProxy :type "/Game/CustomContent/UGC2285067974/Blueprints/Tools/Deathrun_GlobalTool_temporary Object Reference"))
  ;[1 1 1] Dash Fonctionalities
  (set `/Game/CustomContent/UGC2285067974/Blueprints/Tools/Deathrun_GlobalTool_temporary.RibbonOn` true ToolProxy)
  (bind (_direction _dashrate) (`Timeline|DashTimelineServer` :!via `PlayFromStart` :!label _label)
    (:`Update`
      (bind _sweephitresult (`self.K2_SetActorLocation` Owner (+ (* (* (`KismetMathLibrary.Normal` (`KismetMathLibrary.MakeVector` (.x LastInput) (.y LastInput))) (`self.DashRange`)) _dashrate) (`self.K2_GetActorLocation` Owner)) false false)) ; better than add impulse, it's smooth and realy feel like a dash
      (if (`GameplayStatics.BreakHitResult` _sweephitresult)
        (goto _label :!via `Stop`)))
    (:`Finished`
      (set `/Game/CustomContent/UGC2285067974/Blueprints/Tools/Deathrun_GlobalTool_temporary.RibbonOn` false ToolProxy))))

(event `DashClient`
  ;[1 1 1] Dash Fonctionalities
  (bind _charactermoement (`self.GetOwnerCharacterMovement`)
    (:`Output`
      (bind (_direction _dashrate) (`Timeline|DashTimelineClient` :!via `PlayFromStart` :!label _label_2)
        (:`Update`
          (bind _sweephitresult (`self.K2_SetActorLocation` (`self.GetOwner`) (+ (* (* (`KismetMathLibrary.Normal` (`KismetMathLibrary.MakeVector` (.x (`PawnMovementComponent.GetLastInputVector` _charactermoement)) (.y (`PawnMovementComponent.GetLastInputVector` _charactermoement)))) (`self.DashRange`)) _dashrate) (`self.K2_GetActorLocation` (`self.GetOwner`))) false false)) ; better than add impulse, it's smooth and realy feel like a dash
          (if (not (`GameplayStatics.BreakHitResult` _sweephitresult))
            (goto _label_2 :!via `Stop`)))))))

(event `KJModToolProxyInterface.ToolProxy_ShiftModifierPressed`
  (params (pressed :type Boolean))
  ;[1 1 1] Dash Fonctionalities
  (bind _ownerplayerproxy (`self.GetOwnerPlayerProxy`)
    (:`Output`
      (if (and (`|EnumEquality` (`/Game/CustomContent/UGC2285067974/Blueprints/Gamemode/Deathrun_Gamemode.GameState` (`/Game/CustomContent/UGC2285067974/Blueprints/Player/Deathrun_Player.OwningGamemodeProxy` _ownerplayerproxy)) "NewEnumerator5") pressed)
        (bind _tool_used (`self.UseDash`))
        (if _tool_used
          (bind _charactermoement (`self.GetOwnerCharacterMovement`)
            (:`Output`
              (`MovementComponent.StopMovementImmediately` _charactermoement)
              (bind _returnvalue (`PawnMovementComponent.GetLastInputVector` _charactermoement))
              (if (!= _returnvalue (0.0 0.0 0.0))
                (`self.DashServer` _returnvalue (`self.GetOwner`) self)
                (`self.DashClient`)))))))))

(event `Spawn Bait Server`
  (params (Owner :type "Actor Object Reference"))
  (bind _ascharacter (cast `Character` Owner :!pure true))
  ;[1 1 1] Bait Fonctionalities
  (`|SpawnActorFromClass` "/Game/CustomContent/UGC2285067974/Blueprints/Tools/Bait/Bait.Bait_C" (`KismetMathLibrary.MakeTransform` (`self.K2_GetActorLocation` _ascharacter) (`KismetMathLibrary.MakeRotator` 0.0 0.0 (.yaw (`Pawn.GetControlRotation` _ascharacter)))) "Undefined" "OverrideRootScale" Owner null))

(event `KJModToolProxyInterface.ToolProxy_CustomActionPressed`
  (params (cookie :type Integer) (pressed :type Boolean))
  ;[1 1 1] Bait Fonctionalities
  (bind _ownerplayerproxy (`self.GetOwnerPlayerProxy`)
    (:`Output`
      (if (and (== cookie 1) (`|EnumEquality` (`/Game/CustomContent/UGC2285067974/Blueprints/Gamemode/Deathrun_Gamemode.GameState` (`/Game/CustomContent/UGC2285067974/Blueprints/Player/Deathrun_Player.OwningGamemodeProxy` _ownerplayerproxy)) "NewEnumerator5"))
        (bind _tool_used (`self.UseBait`))
        (if _tool_used
          (`self.Spawn Bait Server` (`self.GetOwner`)))))))

(fn `OnRep_CooldownTimeOutBait`
  (bind _ownerplayerproxy (`self.GetOwnerPlayerProxy`)
    (:`Output`
      (`ProgressBar.SetPercent` (`/Game/CustomContent/UGC2285067974/Blueprints/Interface/LocalPlayerHUD.BaitBar` (`/Game/CustomContent/UGC2285067974/Blueprints/Player/Deathrun_Player.LocalPlayerHUD` _ownerplayerproxy)) (/ (`self.CooldownTimeOutBait`) (`self.CooldownBait`))))))

(fn `OnRep_CooldownTimeOutDash`
  (bind _ownerplayerproxy (`self.GetOwnerPlayerProxy`)
    (:`Output`
      (`ProgressBar.SetPercent` (`/Game/CustomContent/UGC2285067974/Blueprints/Interface/LocalPlayerHUD.DashBar` (`/Game/CustomContent/UGC2285067974/Blueprints/Player/Deathrun_Player.LocalPlayerHUD` _ownerplayerproxy)) (/ (`self.CooldownTimeOutDash`) (`self.CooldownDash`))))))

(fn `OnRep_RibbonOn`
  (bind _ownerplayerproxy (`self.GetOwnerPlayerProxy`)
    (:`Output`
      (if (`self.RibbonOn`)
        (bind _dashribbon (`/Game/CustomContent/UGC2285067974/Blueprints/Player/Deathrun_Player.DashRibbon` _ownerplayerproxy))
        (`ActorComponent.Activate` _dashribbon false)
        (else
          (`ActorComponent.Deactivate` _dashribbon))))))

(fn `OnRep_UseCountBait`
  (bind _ownerplayerproxy (`self.GetOwnerPlayerProxy`)
    (:`Output`
      (`Image.SetBrushTintColor` (`/Game/CustomContent/UGC2285067974/Blueprints/Interface/LocalPlayerHUD.BaitBackground` (`/Game/CustomContent/UGC2285067974/Blueprints/Player/Deathrun_Player.LocalPlayerHUD` _ownerplayerproxy)) (select `bool` (== (`self.UseCountBait`) (`self.Max usesBait`)) :`false` (make `SlateColor` (struct :`G` 0.2 :`B` 1.0 :`A` 1.0)) :`true` (make `SlateColor` (struct :`R` 1.0 :`A` 1.0)))))))

(fn `OnRep_UseCountDash`
  (bind _returnvalue (- (`self.Max usesDash`) (`self.UseCountDash`)))
  (bind _returnvalue_2 (== _returnvalue 0))
  (bind _ownerplayerproxy (`self.GetOwnerPlayerProxy`)
    (:`Output`
      (bind _localplayerhud (`/Game/CustomContent/UGC2285067974/Blueprints/Player/Deathrun_Player.LocalPlayerHUD` _ownerplayerproxy))
      (`TextBlock.SetText` (`/Game/CustomContent/UGC2285067974/Blueprints/Interface/LocalPlayerHUD.DashCount` _localplayerhud) (`KismetTextLibrary.Conv_IntToText` _returnvalue))
      (`Image.SetBrushTintColor` (`/Game/CustomContent/UGC2285067974/Blueprints/Interface/LocalPlayerHUD.DashBackground` _localplayerhud) (select `bool` _returnvalue_2 :`false` (make `SlateColor` (struct :`G` 0.2 :`B` 1.0 :`A` 1.0)) :`true` (make `SlateColor` (struct :`R` 1.0 :`A` 1.0))))
      (`Widget.SetVisibility` (`/Game/CustomContent/UGC2285067974/Blueprints/Interface/LocalPlayerHUD.DashCount` _localplayerhud) (select `bool` _returnvalue_2 :`false` "Visible" :`true` "Collapsed" :!type "ESlateVisibility Enum")))))

(fn `UseBait`
  (returns (`Tool used` :type Boolean))
  (if (< (`self.UseCountBait`) (`self.Max usesBait`))
    (set `self.UseCountBait` (+ (`self.UseCountBait`) 1))
    (if (<= (`self.CooldownTimeOutBait`) 0.0)
      (set `self.CooldownTimeOutBait` (`KismetMathLibrary.FMax` 0.0 (`self.CooldownBait`))))
    (return true)
    (else
      (return false))))

(fn `UseDash`
  (returns (`Tool used` :type Boolean))
  (if (< (`self.UseCountDash`) (`self.Max usesDash`))
    (set `self.UseCountDash` (+ (`self.UseCountDash`) 1))
    (if (<= (`self.CooldownTimeOutDash`) 0.0)
      (set `self.CooldownTimeOutDash` (`KismetMathLibrary.FMax` 0.0 (`self.CooldownDash`))))
    (return true)
    (else
      (return false))))

(fn `UserConstructionScript`)